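; BP_TurtleCharacter is a turtle character that handles its own walk animation and its spawn and destruction effects.
; While it moves, Tick calls TecnicalAnimation, which swings the two arm components in opposite pitch between fixed limits, playing a walk sound once per cycle.
; On possession it plays a spawn sound and a brief particle trail.
; When destroyed it plays a finish sound and spawns BP_DestroyEffect at its location.
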(event `self.ReceiveTick`
  (params (DeltaSeconds :type "Float (single-precision)"))
  ;[1 1 1] Анимация передвижения
  (if (> (`KismetMathLibrary.VSize` (`self.GetVelocity`)) 0.0)
    (`self.Tecnical Animation` (* DeltaSeconds 280.0))))

(event `self.ReceivePossessed`
  (params (NewController :type "Controller Object Reference"))
  (bind _particlesystem (`self.ParticleSystem`))
  ;[1 1 1] Анимация появления
  (`GameplayStatics.SpawnSoundAttached` "/Game/MySounds/TurtleSpawnSound.TurtleSpawnSound" (`self.CapsuleComponent`) "None" (0.0 0.0 0.0) (struct) "KeepRelativeOffset" false 1.0 1.0 0.0 null null)
  (`ParticleSystemComponent.BeginTrails` _particlesystem "None" "None" "ETrailWidthMode_FromCentre" 0.0)
  (`KismetSystemLibrary.Delay` 0.3)
  (`ParticleSystemComponent.EndTrails` _particlesystem))

(event `self.ReceiveDestroyed`
  ;[1 1 1] Анимация при уничтожении
  (`GameplayStatics.SpawnSoundAttached` "/Game/MySounds/FinishSound.FinishSound" (`self.CapsuleComponent`) "None" (0.0 0.0 0.0) (struct) "KeepRelativeOffset" false 1.0 1.0 0.0 null null)
  (`|SpawnActorFromClass` "/Game/MyBluePrints/BP_DestroyEffect.BP_DestroyEffect_C" (`KismetMathLibrary.MakeTransform` (`self.K2_GetActorLocation`)) "Undefined" "OverrideRootScale" null null))

(fn `Tecnical Animation`
  (params (Rotation :type "Float (double-precision)"))
  (bind _angle (`self.Angle`))
  (if (`self.ArmIsUp`)
    (bind _output_get (set `self.Angle` (- _angle Rotation)))
    (if (< _output_get -30.0)
      (set `self.ArmIsUp` false)
      (`GameplayStatics.SpawnSoundAttached` "/Game/MySounds/TurtleWalkSound.TurtleWalkSound" (`self.CapsuleComponent`) "None" (0.0 0.0 0.0) (struct) "KeepRelativeOffset" false 1.0 1.0 0.0 null null)
      (else
        (`SceneComponent.K2_SetRelativeTransform` (`self.turtleLeftArm`) (`KismetMathLibrary.MakeTransform` (0.0 0.0 0.0) (`KismetMathLibrary.MakeRotator` 0.0 _angle)) false false :!label _label)
        (`SceneComponent.K2_SetRelativeTransform` (`self.turtleRigtArm`) (`KismetMathLibrary.MakeTransform` (0.0 0.0 0.0) (`KismetMathLibrary.MakeRotator` 0.0 (* _angle -1.0))) false false)))
    (else
      (bind _output_get_2 (set `self.Angle` (+ _angle Rotation)))
      (if (> _output_get_2 30.0)
        (set `self.ArmIsUp` true)
        (else
          (goto _label))))))

(fn `UserConstructionScript`)