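; BP_MyButton is a pressable button that triggers ClickButton on a referenced BP_Gnezdo when something overlaps its Box.
; On overlap it lowers and recolors the Cube, plays audio and makes that call, then restores the Cube after a short delay.
; An IsPress flag blocks repeat presses meanwhile; if the BP_Gnezdo cast fails, the button stays pressed.
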(event `self.Box.OnComponentBeginOverlap`
  (params (OverlappedComponent :type "PrimitiveComponent Object Reference") (OtherActor :type "Actor Object Reference") (OtherComp :type "PrimitiveComponent Object Reference") (OtherBodyIndex :type Integer) (bFromSweep :type Boolean) (SweepResult :type "HitResult Structure (by ref)"))
  (bind _cube (`self.Cube`))
  (if (not (`self.isPress`))
    ;[1 1 1] Нажатие кнопки
    (`SceneComponent.K2_SetRelativeTransform` _cube (`KismetMathLibrary.MakeTransform` (0.0 0.0 0.0) (struct) (1.0 1.0 0.25)) false false)
    (`PrimitiveComponent.SetMaterial` _cube 0 "/Game/MyMaterial/M_MyMaterial.M_MyMaterial")
    (set `self.isPress` true)
    (`AudioComponent.Play` (`self.Audio`) 0.0)
    (bind _asbp_gnezdo (cast `/Game/MyBluePrints/BP_Gnezdo` (`self.GnezdoRef`)))
    (`/Game/MyBluePrints/BP_Gnezdo.ClickButton` _asbp_gnezdo)
    (`KismetSystemLibrary.Delay` 0.3)
    ;[1 1 1] Отжатие кнопки
    (`SceneComponent.K2_SetRelativeTransform` _cube (`KismetMathLibrary.MakeTransform` (0.0 0.0 10.0) (struct) (1.0 1.0 0.25)) false false)
    (`PrimitiveComponent.SetMaterial` _cube 0 "/Game/MyMaterial/M_White_Inst.M_White_Inst")
    (set `self.isPress` false)))

(fn `UserConstructionScript`)